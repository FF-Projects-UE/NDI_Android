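; NDI controller Blueprint for Android that broadcasts and receives NDI video, initialising the plugin and showing a receiver UI shortly after BeginPlay.
; Broadcast creates a sender and pushes frames on a looping timer; a camera render-target send path exists but is disconnected.
; Receive searches the Public group asynchronously and fills the UI's scroll list with a widget per found source.
; EndPlay stops broadcast and reception and releases NDI.
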(event `self.ReceiveBeginPlay`
  (`KismetSystemLibrary.Delay` 2.0)
  (`NDI_AndroidBPLibrary.NDI_Android_Init`)
  (bind _returnvalue (`|CreateWidget` "/NDI_Android/Widgets/UI_NDI_Receiver.UI_NDI_Receiver_C" null self))
  (bind _output_get (set `self.REF_NDI_Receiver_UI` _returnvalue))
  (`UserWidget.AddToViewport` _output_get 0))

(event `self.ReceiveEndPlay`
  (params (EndPlayReason :type "EEndPlayReason Enum" :default "Destroyed"))
  (`|ExecutionSequence`
    (:`then_0`
      (`self.Event_Stop_Broadcast`))
    (:`then_1`
      (`NDI_AndroidBPLibrary.NDI_Android_Release`))
    (:`then_2`
      (`AC_NDI_Receiver.NDI_Android_Receive_Stop` (`self.AC_NDI_Receiver`)))))

(event `Event_Start_Broadcast`
  (bind (_outcode _out_ndi_sender _returnvalue) (`NDI_AndroidBPLibrary.NDI_Android_Sender_Create` "Unreal_Test"))
  (if _returnvalue
    (set `self.REF_NDI_Sender` _out_ndi_sender)
    (`KismetSystemLibrary.K2_SetTimerDelegate` (delegate `Timer_Send_Frames`) 0.1 true)))

(event `Timer_Send_Frames`
  (`NDI_AndroidBPLibrary.NDI_Android_Send_T2D` (`self.REF_NDI_Sender`) null 30.0))

(event `Event_Stop_Broadcast`
  ;[1 1 1] Stop Broadcast
  (`/Engine/EditorBlueprintResources/StandardMacros.IsValid` (`self.REF_NDI_Sender`)
    (:`Is Valid`
      (`NDI_AndroidBPLibrary.NDI_Android_Sender_Release` (`self.REF_NDI_Sender`)))))

(event `Event_Start_Receive`
  (`NDI_AndroidBPLibrary.NDI_Android_Find` (delegate `Delegate_Found`)))

(event `Delegate_Found`
  (params (bIsSuccessfull :type Boolean) (Out_Founds :type "NDI_Android_Found Object Reference") (OutCode :type String))
  (if bIsSuccessfull
    (`PanelWidget.ClearChildren` (`/NDI_Android/Widgets/UI_NDI_Receiver.SCROLL_Sources` (`self.REF_NDI_Receiver_UI`)))
    (for _index (range (`NDI_Android_Found.Source_Count` Out_Founds))
      (bind _returnvalue (`|CreateWidget` "/NDI_Android/Widgets/UI_NDI_Sources.UI_NDI_Sources_C" null _index Out_Founds (`self.REF_NDI_Receiver_UI`) self))
      (`PanelWidget.AddChild` (`/NDI_Android/Widgets/UI_NDI_Receiver.SCROLL_Sources` (`self.REF_NDI_Receiver_UI`)) _returnvalue)
      (`UserWidget.SetPadding` _returnvalue (make `Margin` 5.0 5.0 5.0 5.0)))))

(fn `UserConstructionScript`)